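; BP_DuraMainMenu is the main menu scene actor that plays menu music and shows the WBP_MainMenu widget with UI-only input and a visible cursor.
; Each tick it bobs the FireBall vertically around its starting location using a sine of an accumulated, wrapping time value scaled by Amplitude.
; It also continuously spins the MagicCircleDecal around its roll axis at a configurable rate.
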(event `self.ReceiveBeginPlay`
  (bind _returnvalue (`GameplayStatics.GetPlayerController` 0))
  (set `self.InitialFireballLocation` (`SceneComponent.K2_GetComponentLocation` (`self.FireBall`)))
  (`GameplayStatics.PlaySound2D` "/Game/Assets/Sounds/Music/Music_MainMenu.Music_MainMenu" 1.0 1.0 0.0 null null)
  (bind _returnvalue_2 (`|CreateWidget` "/Game/Blueprints/UI/MainMenu/WBP_MainMenu.WBP_MainMenu_C"))
  (`UserWidget.AddToViewport` _returnvalue_2 0)
  (`WidgetBlueprintLibrary.SetInputMode_UIOnlyEx` _returnvalue _returnvalue_2)
  (set `PlayerController.bShowMouseCursor` true _returnvalue))

(event `self.ReceiveTick`
  (params (DeltaSeconds :type "Float (single-precision)"))
  (`self.UpdateTime` DeltaSeconds)
  (`SceneComponent.K2_SetWorldLocation` (`self.FireBall`) (+ (`self.InitialFireballLocation`) (`KismetMathLibrary.MakeVector` 0.0 0.0 (`self.SinTime`))) false false)
  (`SceneComponent.K2_AddLocalRotation` (`self.MagicCircleDecal`) (`KismetMathLibrary.MakeRotator` (* (`GameplayStatics.GetWorldDeltaSeconds`) (`self.Magic Circle Rotation Rate`))) false false))

(fn `SinTime`
  (returns (ReturnValue :type "Float (double-precision)"))
  (return (* (`KismetMathLibrary.Sin` (`self.Time`)) (`self.Amplitude`))))

(fn `UpdateTime`
  (params (B :type "Float (double-precision)"))
  (bind _output_get (set `self.Time` (+ (`self.Time`) B)))
  (if (> _output_get (* (`KismetMathLibrary.GetPI`) 2.0))
    (set `self.Time` 0.0)))

(fn `UserConstructionScript`)