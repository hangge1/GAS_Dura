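; Enemy ranged attack gameplay ability that turns the avatar toward its combat target and fires a projectile.
; It gets the target and attack montages through interface messages on the avatar, then plays a random tagged montage.
; A gameplay event triggers SpawnProjectile with the combat socket location for that montage's tag, then ends the ability.
; The montage keeps playing after the ability ends; montage completion, interruption or cancellation also ends it.
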(event `self.K2_ActivateAbility`
  (bind _returnvalue (`self.GetAvatarActorFromActorInfo`))
  (bind (_montage _montagetag) (break `TaggedMontage` (`self.TaggedMontage`)))
  (bind _returnvalue_2 (message `EnemyInterface.GetCombatTarget` _returnvalue))
  (message `CombatInterface.UpdateFacingTarget` _returnvalue (`Actor.K2_GetActorLocation` _returnvalue_2))
  (bind _returnvalue_3 (message `CombatInterface.GetAttackMontages` (`self.GetAvatarActorFromActorInfo`)))
  (set `self.TaggedMontage` (`self.GetRandomTaggedMontageFromArray` _returnvalue_3))
  (`AbilityTask_PlayMontageAndWait.CreatePlayMontageAndWaitProxy` "None" _montage 1.0 "None" false
    (:`then`
      (`AbilityTask_WaitGameplayEvent.WaitGameplayEvent` (struct) null
        (:`then`
          (bind _returnvalue_4 (message `CombatInterface.GetCombatSocketLocation` (`self.GetAvatarActorFromActorInfo`) _montagetag))
          (`self.SpawnProjectile` _returnvalue_4)
          (`self.K2_EndAbility`))))
    (:`OnCompleted`
      (`self.K2_EndAbility` :!label _label))
    (:`OnInterrupted`
      (goto _label))
    (:`OnCancelled`
      (goto _label))))