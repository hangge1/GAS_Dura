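; BP_SlingshorRock is a rock actor for an enemy ability, apparently a slingshot projectile, that tumbles while it exists.
; BeginPlay picks random pitch, roll and yaw rates, which Tick scales by delta time to spin the actor in local space.
; After a brief delay, BeginPlay sets the Sphere's collision to query-only if the component is valid.
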(event `self.ReceiveBeginPlay`
  (bind _returnvalue (`KismetMathLibrary.RandomFloatInRange` 0.0 360.0))
  (set `self.PitchRandom` _returnvalue)
  (set `self.RollRandom` _returnvalue)
  (set `self.YawRandom` _returnvalue)
  (`KismetSystemLibrary.Delay` 0.1)
  (bind _sphere (`self.Sphere`)
    (:`then`
      (`PrimitiveComponent.SetCollisionEnabled` _sphere "QueryOnly"))
    (:`else`)))

(event `self.ReceiveTick`
  (params (DeltaSeconds :type "Float (single-precision)"))
  (`self.K2_AddActorLocalRotation` (`KismetMathLibrary.MakeRotator` (* DeltaSeconds (`self.RollRandom`)) (* DeltaSeconds (`self.PitchRandom`)) (* DeltaSeconds (`self.YawRandom`)))))

(fn `UserConstructionScript`)