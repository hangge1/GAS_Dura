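; Gameplay ability for enemy melee attacks: faces the combat target and plays a random tagged attack montage from the avatar's combat interface.
; The montage's gameplay event triggers a small radius query at the tagged socket, damaging and applying a damage effect to every non-friendly live player found.
; If anything is hit, a MeleeImpact gameplay cue fires at the socket.
; The ability ends after that event or when the montage finishes or is interrupted.
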(event `self.K2_ActivateAbility`
  (bind (_montage _montagetag) (break `TaggedMontage` (`self.TaggedMontage`)))
  (set `self.HasHitTarget` false)
  (bind _ascombat_interface (cast `CombatInterface` (`self.GetAvatarActorFromActorInfo`))
    (:`then`
      (set `self.CombatInterface` _ascombat_interface)
      (`self.UpdateFacingTarget`)
      (`self.GetRandomTaggedMontage`)
      (`AbilityTask_PlayMontageAndWait.CreatePlayMontageAndWaitProxy` "None" _montage 1.0 "None" false
        (:`then`
          (`AbilityTask_WaitGameplayEvent.WaitGameplayEvent` _montagetag null
            (:`EventReceived`
              (`self.GetCombatSocketLocation`)
              (bind _combatliveplayers (`self.GetCombatLivePlayers`))
              (for _array_element _combatliveplayers
                (`self.CauseTargetDamage` _array_element))
              (`self.ExecuteImpactEffect`)
              (`self.K2_EndAbility`))))
        (:`OnCompleted`
          (`self.K2_EndAbility` :!label _label))
        (:`OnInterrupted`
          (goto _label))
        (:`OnCancelled`
          (goto _label))))
    (:`CastFailed`
      (`self.K2_EndAbility`))))

(fn `CauseTargetDamage`
  (params (TargetActor :type "Actor Object Reference"))
  (locals (Target :type "Actor Object Reference"))
  (set `local.Target` TargetActor)
  (if (`DuraAbilitySystemLibrary.IsNotFriend` (`local.Target`) (`self.GetAvatarActorFromActorInfo`))
    (`self.CauseDamage` (`local.Target`))
    (set `self.HasHitTarget` true)
    (`DuraAbilitySystemLibrary.ApplyDamageEffect` (`self.MakeDamageEffectParamsFromClassDefaults` (`local.Target`)))))

(fn `ExecuteImpactEffect`
  (if (`self.HasHitTarget`)
    (bind _returnvalue (message `EnemyInterface.GetCombatTarget` (`self.GetAvatarActorFromActorInfo`)))
    (`self.K2_ExecuteGameplayCueWithParams` (struct :`TagName` "GameplayCue.MeleeImpact") (`AbilitySystemBlueprintLibrary.MakeGameplayCueParameters` 0.0 0.0 (struct) (struct) (struct) (`BlueprintGameplayTagLibrary.MakeGameplayTagContainerFromTag` (`.MontageTag` (break `TaggedMontage` (`self.TaggedMontage`)))) (struct) (`self.CombatSocketLocation`) (0.0 0.0 0.0) null (`self.GetAvatarActorFromActorInfo`) _returnvalue))))

(fn `GetCombatLivePlayers`
  (returns (CombatLivePlayers :type "Array of Actor Object Reference"))
  (bind _returnvalue (`self.GetAvatarActorFromActorInfo`))
  (bind _outoverlappingactors (`DuraAbilitySystemLibrary.GetLivePlayersWithinRadius` _returnvalue (`|MakeArray` _returnvalue) 45.0 (`self.CombatSocketLocation`)))
  (return _outoverlappingactors))

(fn `GetCombatSocketLocation`
  (bind _returnvalue (message `CombatInterface.GetCombatSocketLocation` (`self.GetAvatarActorFromActorInfo`) (`.SocketTag` (break `TaggedMontage` (`self.TaggedMontage`)))))
  (set `self.CombatSocketLocation` _returnvalue))

(fn `GetRandomTaggedMontage`
  (bind _returnvalue (message `CombatInterface.GetAttackMontages` (`self.GetAvatarActorFromActorInfo`)))
  (set `self.TaggedMontage` (`self.GetRandomTaggedMontageFromArray` _returnvalue)))

(fn `UpdateFacingTarget`
  (bind _returnvalue (message `EnemyInterface.GetCombatTarget` (`self.GetAvatarActorFromActorInfo`)))
  (`CombatInterface.UpdateFacingTarget` (`self.CombatInterface`) (`Actor.K2_GetActorLocation` _returnvalue)))