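; BP_FireBolt is the projectile actor for the Fire Bolt ability.
; It switches its Sphere to query-only collision after a short delay from spawn.
; Each tick it compares its position to the previous frame's and, if it moved less than a minimum distance, plays the impact sound and Niagara explosion, then destroys itself.
; This graph applies no damage and leaves the overlap event empty.
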(event `self.ReceiveBeginPlay`
  (`KismetSystemLibrary.Delay` 0.2)
  (bind _sphere (`self.Sphere`)
    (:`then`
      (`PrimitiveComponent.SetCollisionEnabled` _sphere "QueryOnly"))
    (:`else`)))

(event `self.ReceiveTick`
  (params (DeltaSeconds :type "Float (single-precision)"))
  (`self.MakeGoKaboomIfNoMove`))

(fn `MakeGoKaboomIfNoMove`
  (set `self.LocationLastFrame` (`self.LocationThisFrame`))
  (set `self.LocationThisFrame` (`self.K2_GetActorLocation`))
  (if (< (`KismetMathLibrary.VSize` (- (`self.LocationThisFrame`) (`self.LocationLastFrame`))) (`self.MinDistancePerFrame`))
    (`GameplayStatics.SpawnSoundAtLocation` "/Game/Assets/Sounds/Abilities/FireBolt/sfx_FireBolt_Impact.sfx_FireBolt_Impact" (`self.LocationThisFrame`) (struct) 1.0 1.0 0.0 null null)
    (`NiagaraFunctionLibrary.SpawnSystemAtLocation` "/Game/Assets/Effects/Projectiles/FireExplosion/NS_FireExplosion.NS_FireExplosion" (`self.LocationThisFrame`))
    (`self.K2_DestroyActor`)))

(fn `UserConstructionScript`)