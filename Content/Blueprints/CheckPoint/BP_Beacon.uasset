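; BP_Beacon is a checkpoint beacon that lights up when an actor implementing PlayerInterface enters its sphere.
; The overlap calls HandleGlowEffects, defined outside these graphs, and marks the beacon as Reached.
; The CheckpointReached event plays a timeline that drives the Glow parameter of the supplied dynamic material, scaled by GlowFactor.
; The construction script turns CallOverlapCallback off.
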(event `self.Sphere.OnComponentBeginOverlap`
  (params (OverlappedComponent :type "PrimitiveComponent Object Reference") (OtherActor :type "Actor Object Reference") (OtherComp :type "PrimitiveComponent Object Reference") (OtherBodyIndex :type Integer) (bFromSweep :type Boolean) (SweepResult :type "HitResult Structure (by ref)"))
  (if (`KismetSystemLibrary.DoesImplementInterface` OtherActor "/Script/Dura.PlayerInterface")
    (`self.HandleGlowEffects`)
    (set `self.bReached` true)))

(event `self.CheckpointReached`
  (params (MaterialInstanceDynamic :type "MaterialInstanceDynamic Object Reference"))
  (bind (_direction _beacontrack) (`Timeline|BeaconTimeline`)
    (:`Update`
      (`MaterialInstanceDynamic.SetScalarParameterValue` MaterialInstanceDynamic "Glow" (* _beacontrack (`self.GlowFactor`))))))

(fn `UserConstructionScript`
  (set `self.bCallOverlapCallback` false))