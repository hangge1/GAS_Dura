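; BP_FlamePillar is a flame pillar actor whose fire light flickers continuously.
; On BeginPlay it randomly picks one of two FlameIntensity timelines and plays it from the start, choosing again whenever one finishes.
; Each timeline update passes its curve value to ScaleFlameIntensity, which multiplies it by BaseIntensity to set the FireLight intensity.
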(event `self.ReceiveBeginPlay`
  (`self.ChooseTimeline`))

(event `ChooseTimeline`
  (switch `int` (`KismetMathLibrary.RandomIntegerInRange` 0 1)
    (:`0`
      (`self.StartFlame1`))
    (:`1`
      (`self.StartFlame2`))))

(event `StartFlame1`
  (bind (_direction _flameintensity) (`Timeline|FlameIntensity_1` :!via `PlayFromStart`)
    (:`Update`
      (`self.ScaleFlameIntensity` _flameintensity))
    (:`Finished`
      (`self.ChooseTimeline`))))

(event `StartFlame2`
  (bind (_direction _flameintensity) (`Timeline|FlameIntensity_2` :!via `PlayFromStart`)
    (:`Update`
      (`self.ScaleFlameIntensity` _flameintensity))
    (:`Finished`
      (`self.ChooseTimeline`))))

(fn `ScaleFlameIntensity`
  (params (Intensity :type "Float (double-precision)"))
  (`LightComponent.SetIntensity` (`self.FireLight`) (* Intensity (`self.BaseIntensity`))))

(fn `UserConstructionScript`)